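; BP_Battery is a collectible pickup that adds a battery to the ThirdPersonCharacter.
; Overlapping BatteryMesh calls AddBattery, plays a pop sound and destroys the actor.
; Entering MagneticField while the character's magnet is active starts a timeline that pulls the battery toward player 0.
; Each update moves it with VInterpTo plus the timeline's Slide offset, without sweeping.
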(event `self.BatteryMesh.OnComponentBeginOverlap`
  (params (OverlappedComponent :type "PrimitiveComponent Object Reference") (OtherActor :type "Actor Object Reference") (OtherComp :type "PrimitiveComponent Object Reference") (OtherBodyIndex :type Integer) (bFromSweep :type Boolean) (SweepResult :type "HitResult Structure (by ref)"))
  (bind _asthird_person_character (cast `/Game/ThirdPersonBP/Blueprints/ThirdPersonCharacter` OtherActor))
  (`/Game/ThirdPersonBP/Blueprints/ThirdPersonCharacter.AddBattery` _asthird_person_character)
  (`GameplayStatics.PlaySoundAtLocation` "/Game/Sounds/mixkit-electric-pop-2365.mixkit-electric-pop-2365" (`self.K2_GetActorLocation`) (struct) 1.0 1.0 0.0 null null null)
  (`self.K2_DestroyActor`))

(event `self.MagneticField.OnComponentBeginOverlap`
  (params (OverlappedComponent :type "PrimitiveComponent Object Reference") (OtherActor :type "Actor Object Reference") (OtherComp :type "PrimitiveComponent Object Reference") (OtherBodyIndex :type Integer) (bFromSweep :type Boolean) (SweepResult :type "HitResult Structure (by ref)"))
  (bind _asthird_person_character (cast `/Game/ThirdPersonBP/Blueprints/ThirdPersonCharacter` OtherActor))
  (bind _newparam (`/Game/ThirdPersonBP/Blueprints/ThirdPersonCharacter.IsMagnetActive` _asthird_person_character))
  (if _newparam
    (bind (_direction _slide) (`Timeline|Timeline_0` :!via `PlayFromStart`)
      (:`Update`
        (`self.K2_SetActorLocation` (+ _slide (`KismetMathLibrary.VInterpTo` (.location (`self.GetTransform`)) (`self.K2_GetActorLocation` (`GameplayStatics.GetPlayerCharacter` 0)) (`GameplayStatics.GetWorldDeltaSeconds`) 15.0)))))))

(fn `UserConstructionScript`)