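; Base floor tile actor for an endless-runner level, which spawns track ahead and removes itself once passed.
; When the player character overlaps EndTrigger, it raises the character's speed and tile count, asks the game mode to add floor tiles, then destroys itself after a short delay.
; GetAttachTransform exposes the AttachPoint transform as a connection point for another tile.
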(event `self.EndTrigger.OnComponentBeginOverlap`
  (params (OverlappedComponent :type "PrimitiveComponent Object Reference") (OtherActor :type "Actor Object Reference") (OtherComp :type "PrimitiveComponent Object Reference") (OtherBodyIndex :type Integer) (bFromSweep :type Boolean) (SweepResult :type "HitResult Structure (by ref)"))
  (bind _asthird_person_character (cast `/Game/ThirdPersonBP/Blueprints/ThirdPersonCharacter` OtherActor))
  (`/Game/ThirdPersonBP/Blueprints/ThirdPersonCharacter.IncreaseSpeed` _asthird_person_character)
  (`/Game/ThirdPersonBP/Blueprints/ThirdPersonCharacter.AddTileCount` _asthird_person_character)
  (bind _asthird_person_game_mode (cast `/Game/ThirdPersonBP/Blueprints/ThirdPersonGameMode` (`GameplayStatics.GetGameMode`)))
  (`/Game/ThirdPersonBP/Blueprints/ThirdPersonGameMode.AddFloorTile` _asthird_person_game_mode 2)
  (`KismetSystemLibrary.Delay` 2.0)
  (`self.K2_DestroyActor`))

(fn `GetAttachTransform`
  (returns (AttachTransform :type "Transform Structure"))
  (return (`SceneComponent.K2_GetComponentToWorld` (`self.AttachPoint`))))

(fn `UserConstructionScript`)