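; Level tile that randomly populates itself with barriers, rows of batteries and a magnet, all as child actors.
; The Construction Script caches left, center and right attach points, then randomly fills one, two or all three for barriers and, independently, batteries.
; Single and paired barriers randomly pick big or small, while full rows skip that roll.
; Batteries repeat along X in random-length lines, and the magnet lands randomly inside the MagnetArea box.
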(fn `LoopBatteryFromPoint`
  (params (AttachPoint :type "Vector Structure"))
  (locals (AttachPointX :type "Float (double-precision)") (AttachPointY :type "Float (double-precision)" :default 0.0) (AttachPointZ :type "Float (double-precision)" :default 0.0))
  (set `local.AttachPointX` (.x AttachPoint))
  (set `local.AttachPointY` (.y AttachPoint))
  (set `local.AttachPointZ` (.z AttachPoint))
  (for _ (range (+ (`KismetMathLibrary.RandomIntegerInRange` 2 9) 1))
    (`AddComponent|NODE_AddChildActorComponent-19` :`RelativeTransform` (`KismetMathLibrary.Conv_VectorToTransform` (`KismetMathLibrary.MakeVector` (`local.AttachPointX`) (`local.AttachPointY`) (`local.AttachPointZ`))))
    (set `local.AttachPointX` (+ (`local.AttachPointX`) 100.0))))

(fn `RandomGenarateBarrier`
  (params (AttachPoint :type "Vector Structure"))
  (switch `int` (`KismetMathLibrary.RandomIntegerInRange` 0 1)
    (:`Default`
      ;[1 1 1] Spawn Small Barrier
      (`AddComponent|NODE_AddChildActorComponent-21` :`RelativeTransform` (`KismetMathLibrary.Conv_VectorToTransform` AttachPoint) :!label _label))
    (:`0`
      ;[1 1 1] Spawn Big Barrier
      (`AddComponent|NODE_AddChildActorComponent-22` :`RelativeTransform` (`KismetMathLibrary.Conv_VectorToTransform` AttachPoint)))
    (:`1`
      (goto _label))))

(fn `SetBarrierAttachPoint`
  (bind _barrierattachpoint (`self.BarrierAttachPoint`))
  (`KismetArrayLibrary.Array_Add` _barrierattachpoint (`SceneComponent.RelativeLocation` (`self.BarrierAttachLeft`)))
  (`KismetArrayLibrary.Array_Add` _barrierattachpoint (`SceneComponent.RelativeLocation` (`self.BarrierAttachCenter`)))
  (`KismetArrayLibrary.Array_Add` _barrierattachpoint (`SceneComponent.RelativeLocation` (`self.BarrierAttachRight`))))

(fn `SetBatteryAttachPoint`
  (bind _batteryattachpoint (`self.BatteryAttachPoint`))
  (`KismetArrayLibrary.Array_Add` _batteryattachpoint (`SceneComponent.RelativeLocation` (`self.BatteryAttachLeft`)))
  (`KismetArrayLibrary.Array_Add` _batteryattachpoint (`SceneComponent.RelativeLocation` (`self.BatteryAttachCenter`)))
  (`KismetArrayLibrary.Array_Add` _batteryattachpoint (`SceneComponent.RelativeLocation` (`self.BatteryAttachRight`))))

(fn `Spawn Batteries`
  (switch `int` (`KismetMathLibrary.RandomIntegerInRange` 0 2)
    (:`Default`
      (`self.SpawnBatteryOnTwoPoints` :!label _label))
    (:`0`
      (`self.SpawnBatteryOnThreePoints`))
    (:`1`
      (goto _label))
    (:`2`
      (`self.SpawnBatteryOnSinglePoint`))))

(fn `SpawnBarrier`
  (switch `int` (`KismetMathLibrary.RandomIntegerInRange` 0 2)
    (:`0`
      (`self.SpawnBarrierOnThreePoints`))
    (:`1`
      (`self.SpawnBarrierOnTwoPoints`))
    (:`2`
      (`self.SpawnBarrierOnSInglePoint`))))

(fn `SpawnBarrierOnCenterPoint`
  (`self.RandomGenarateBarrier` (`|GetArrayItem` (`self.BarrierAttachPoint`) 1)))

(fn `SpawnBarrierOnLeftPoint`
  (`self.RandomGenarateBarrier` (`|GetArrayItem` (`self.BarrierAttachPoint`))))

(fn `SpawnBarrierOnRightPoint`
  (`self.RandomGenarateBarrier` (`|GetArrayItem` (`self.BarrierAttachPoint`) 2)))

(fn `SpawnBarrierOnSInglePoint`
  (switch `int` (`KismetMathLibrary.RandomIntegerInRange` 0 2)
    (:`Default`
      (`self.SpawnBarrierOnCenterPoint` :!label _label))
    (:`0`
      (`self.SpawnBarrierOnLeftPoint`))
    (:`1`
      (goto _label))
    (:`2`
      (`self.SpawnBarrierOnRightPoint`))))

(fn `SpawnBarrierOnThreePoints`
  (for _array_element (`self.BarrierAttachPoint`)
    (`AddComponent|NODE_AddChildActorComponent-1` :`RelativeTransform` (`KismetMathLibrary.Conv_VectorToTransform` _array_element))))

(fn `SpawnBarrierOnTwoPoints`
  (switch `int` (`KismetMathLibrary.RandomIntegerInRange` 0 2)
    (:`Default`
      ;[1 1 1] Left and Right
      (`self.SpawnBarrierOnLeftPoint` :!label _label)
      (`self.SpawnBarrierOnRightPoint`))
    (:`0`
      ;[1 1 1] Left and Center
      (`self.SpawnBarrierOnLeftPoint`)
      (`self.SpawnBarrierOnCenterPoint`))
    (:`1`
      (goto _label))
    (:`2`
      ;[1 1 1] Center and Right
      (`self.SpawnBarrierOnCenterPoint`)
      (`self.SpawnBarrierOnRightPoint`))))

(fn `SpawnBatteryOnCenterPoint`
  (`self.LoopBatteryFromPoint` (`|GetArrayItem` (`self.BatteryAttachPoint`) 1)))

(fn `SpawnBatteryOnLeftPoint`
  (`self.LoopBatteryFromPoint` (`|GetArrayItem` (`self.BatteryAttachPoint`))))

(fn `SpawnBatteryOnRightPoint`
  (`self.LoopBatteryFromPoint` (`|GetArrayItem` (`self.BatteryAttachPoint`) 2)))

(fn `SpawnBatteryOnSinglePoint`
  (switch `int` (`KismetMathLibrary.RandomIntegerInRange` 0 2)
    (:`Default`
      (`self.SpawnBatteryOnCenterPoint` :!label _label))
    (:`0`
      (`self.SpawnBatteryOnLeftPoint`))
    (:`1`
      (goto _label))
    (:`2`
      (`self.SpawnBatteryOnRightPoint`))))

(fn `SpawnBatteryOnThreePoints`
  (`self.SpawnBatteryOnLeftPoint`)
  (`self.SpawnBatteryOnCenterPoint`)
  (`self.SpawnBatteryOnRightPoint`))

(fn `SpawnBatteryOnTwoPoints`
  (switch `int` (`KismetMathLibrary.RandomIntegerInRange` 0 2)
    (:`0`
      ;[1 1 1] Left and Center
      (`self.SpawnBatteryOnLeftPoint`)
      (`self.SpawnBatteryOnCenterPoint`))
    (:`1`
      ;[1 1 1] Left and Right
      (`self.SpawnBatteryOnLeftPoint`)
      (`self.SpawnBatteryOnRightPoint`))
    (:`2`
      ;[1 1 1] Center and Right
      (`self.SpawnBatteryOnCenterPoint`)
      (`self.SpawnBatteryOnRightPoint`))))

(fn `SpawnMagnet`
  (bind _magnetarea (`self.MagnetArea`))
  (`AddComponent|NODE_AddChildActorComponent-14` :`RelativeTransform` (`KismetMathLibrary.Conv_VectorToTransform` (`KismetMathLibrary.RandomPointInBoundingBox` (`SceneComponent.RelativeLocation` _magnetarea) (`BoxComponent.BoxExtent` _magnetarea)))))

(fn `UserConstructionScript`
  (`self.SetBarrierAttachPoint`)
  (`self.SpawnBarrier`)
  (`self.SetBatteryAttachPoint`)
  (`self.Spawn Batteries`)
  (`self.SpawnMagnet`))