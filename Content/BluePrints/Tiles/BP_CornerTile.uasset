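; BP_CornerTile is a corner tile that lets the player character turn and kills it on a wall hit.
; Overlapping TurnBox sets CanTurn to true on the ThirdPersonCharacter, and nothing here resets it.
; A hit on RightWall1 calls Death on that character, and both handlers ignore other actors through a cast.
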(event `self.TurnBox.OnComponentBeginOverlap`
  (params (OverlappedComponent :type "PrimitiveComponent Object Reference") (OtherActor :type "Actor Object Reference") (OtherComp :type "PrimitiveComponent Object Reference") (OtherBodyIndex :type Integer) (bFromSweep :type Boolean) (SweepResult :type "HitResult Structure (by ref)"))
  (bind _asthird_person_character (cast `/Game/ThirdPersonBP/Blueprints/ThirdPersonCharacter` OtherActor))
  (set `/Game/ThirdPersonBP/Blueprints/ThirdPersonCharacter.canTurn` true _asthird_person_character))

(event `self.RightWall1.OnComponentHit`
  (params (HitComponent :type "PrimitiveComponent Object Reference") (OtherActor :type "Actor Object Reference") (OtherComp :type "PrimitiveComponent Object Reference") (NormalImpulse :type "Vector Structure") (Hit :type "HitResult Structure (by ref)"))
  (bind _asthird_person_character (cast `/Game/ThirdPersonBP/Blueprints/ThirdPersonCharacter` OtherActor))
  (`/Game/ThirdPersonBP/Blueprints/ThirdPersonCharacter.Death` _asthird_person_character))

(fn `UserConstructionScript`
  (`parent.UserConstructionScript`))